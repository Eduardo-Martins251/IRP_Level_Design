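; BP_BreakableLight is a light hazard that goes dark with a bulb-breaking sound when the player walks into its trigger box.
; If CanFlicker is set, a timeline starts on BeginPlay and drives the referenced TargetLight's intensity from its Flicker track.
; On player overlap it plays the sound at the light, hides the light's root, disables the box collision so it fires once, and stops the flicker.
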(event `self.ReceiveBeginPlay`
  (if (`self.CanFlicker`)
    (bind (_direction _flicker) (`Timeline|Timeline` :!label _label)
      (:`Update`
        (`LightComponent.SetIntensity` (`Light.LightComponent` (`self.TargetLight`)) (* _flicker 1000.0))))))

(event `self.Box.OnComponentBeginOverlap`
  (params (OverlappedComponent :type "PrimitiveComponent Object Reference") (OtherActor :type "Actor Object Reference") (OtherComp :type "PrimitiveComponent Object Reference") (OtherBodyIndex :type Integer) (bFromSweep :type Boolean) (SweepResult :type "HitResult Structure (by ref)"))
  (cast `/Game/Blueprints/BP_Player` OtherActor)
  (`GameplayStatics.PlaySoundAtLocation` "/Game/Audio/kakaist-lightbulb-break-sfx-320646.kakaist-lightbulb-break-sfx-320646" (`SceneComponent.K2_GetComponentLocation` (`Actor.RootComponent` (`self.TargetLight`))) (struct) 1.0 1.0 0.0 null null null null)
  (`SceneComponent.SetVisibility` (`Actor.RootComponent` (`self.TargetLight`)) false false)
  (`PrimitiveComponent.SetCollisionEnabled` (`self.Box`) "NoCollision")
  (goto _label :!via `Stop`))

(fn `UserConstructionScript`)